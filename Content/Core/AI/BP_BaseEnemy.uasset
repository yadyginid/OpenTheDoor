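; Base enemy Blueprint that deals attack damage through an overlap sphere using the Gameplay Ability System.
; At BeginPlay it listens for gameplay events that enable and disable the sphere's collision, opening and closing the damage window.
; Any other overlapping actor with an Ability System Component gets GE_Damage applied to itself through that component, with no team filtering.
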(event OnComponentBeginOverlap(DamageSphereOverlap)
  (params (OverlappedComponent :type Primitive%20Component%20Object%20Reference) (OtherActor :type Actor%20Object%20Reference) (OtherComp :type Primitive%20Component%20Object%20Reference) (OtherBodyIndex :type Integer) (bFromSweep :type Boolean) (SweepResult :type Hit%20Result%20Structure%20%28by%20ref%29))
  (bind _returnvalue (Ability|GetAbilitySystemComponent OtherActor))
  (if (!= OtherActor self)
    (Utilities|IsValid _returnvalue
      (:Is%20Valid
        (GameplayEffects|ApplyGameplayEffectToSelf :self _returnvalue :GameplayEffectClass "/Game/Core/GAS/Effects/Damage/GE_Damage.GE_Damage_C" :Level 1.0)))))

(event EventBeginPlay
  (Ability|Async|WaitGameplayEventToActor 0 "(TagName=\"Events.EnableAttackCollision\")"
    (:then
      (Ability|Async|WaitGameplayEventToActor 0 "(TagName=\"Events.DisableAttackCollosion\")"
        (:EventReceived
          (Collision|SetCollisionEnabled (Variables|Default|GetDamageSphereOverlap) "NoCollision"))))
    (:EventReceived
      (Collision|SetCollisionEnabled (Variables|Default|GetDamageSphereOverlap) "QueryOnly"))))

(fn ConstructionScript)