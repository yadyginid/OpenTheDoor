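; GA_Sprint is a gameplay ability that makes BP_PlayerCharacter sprint by raising its movement speed.
; On activation it caches the character's MaxWalkSpeed, applies SprintSpeed and sets the Sprint flag to true.
; It waits for the Input.SprintReleased gameplay event, then restores the cached speed.
; The release branch also sets Sprint to true rather than clearing it, and the graph never calls EndAbility.
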(event Ability|EventActivateAbility
  (bind _returnvalue (Ability|GetAvatarActorfromActorInfo))
  (Utilities|IsValid _returnvalue
    (:Is%20Valid
      (bind _asbp_player_character (Utilities|Casting|CastToBP_PlayerCharacter _returnvalue))
      (bind _output_get (Variables|Default|SetAs%20BP%20Third%20Person%20Character _asbp_player_character))
      (Utilities|IsValid (Variables|/Script/Engine.Character|GetCharacterMovement _output_get)
        (:Is%20Valid
          (Variables|Default|SetCharacter%20Movement (Variables|/Script/Engine.Character|GetCharacterMovement _output_get))
          (Variables|Default|SetMax%20Walk%20Speed (Variables|/Script/Engine.CharacterMovementComponent|GetMaxWalkSpeed (Variables|Default|GetCharacter%20Movement)))
          (Variables|/Script/Engine.CharacterMovementComponent|SetMaxWalkSpeed (Variables|Default|GetCharacter%20Movement) (Variables|Default|GetSprintSpeed))
          (Variables|/Game/Core/Player/BP_PlayerCharacter.BP_PlayerCharacter_C|SetSprint (Variables|Default|GetAs%20BP%20Third%20Person%20Character) true)
          (Ability|Tasks|WaitGameplayEvent "(TagName=\"Input.SprintReleased\")" 0
            (:EventReceived
              (Variables|/Script/Engine.CharacterMovementComponent|SetMaxWalkSpeed (Variables|Default|GetCharacter%20Movement) (Variables|Default|GetMax%20Walk%20Speed))
              (Variables|/Game/Core/Player/BP_PlayerCharacter.BP_PlayerCharacter_C|SetSprint (Variables|Default|GetAs%20BP%20Third%20Person%20Character) true))))))))