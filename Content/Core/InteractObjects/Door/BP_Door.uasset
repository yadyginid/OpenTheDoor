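; BP_Door is an interactable double door that swings open or closed when the player interacts with it.
; BPIInteract toggles IsOpen and calls Open or Close, which use separate timelines, one played from start and the other reversed.
; Timeline output sets the yaw of RightDoor and the mirrored yaw of LeftDoor.
; BPIShow and BPIHide toggle a widget that starts hidden.
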(event Custom|Open
  (bind _rotation (Timeline|PlayRightDoor PlayFromStart)
    (:Update
      (Transformation|SetRelativeRotation (Variables|Default|GetRightDoor) (Math|Rotator|MakeRotator 0.0 0.0 _rotation) false false)
      (Transformation|SetRelativeRotation (Variables|Default|GetLeftDoor) (Math|Rotator|MakeRotator 0.0 0.0 (* _rotation -1.0)) false false))))

(event Custom|Close
  (bind _rotation (Timeline|Timeline Reverse)
    (:Update
      (Transformation|SetRelativeRotation (Variables|Default|GetRightDoor) (Math|Rotator|MakeRotator 0.0 0.0 _rotation) false false)
      (Transformation|SetRelativeRotation (Variables|Default|GetLeftDoor) (Math|Rotator|MakeRotator 0.0 0.0 (* _rotation -1.0)) false false))))

(event EventBPIInteract
  (if (not (Variables|Default|GetIsOpen))
    (CallFunction|Open)
    (Variables|Default|SetIsOpen true)
    (else
      (CallFunction|Close)
      (Variables|Default|SetIsOpen false))))

(event EventBPIShow
  (Rendering|SetVisibility (Variables|Default|GetWidget) true false))

(event EventBeginPlay
  (Rendering|SetVisibility (Variables|Default|GetWidget) false false))

(event EventBPIHide
  (Rendering|SetVisibility (Variables|Default|GetWidget) false false))

(fn ConstructionScript)