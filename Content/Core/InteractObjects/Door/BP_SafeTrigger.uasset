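; BP_SafeTrigger is a trigger actor that grants the player a safe-state Gameplay Effect between an entry and an exit overlap.
; Overlapping Enter applies GE_Safe through the PlayerCharacter's Ability System Component and stores the active effect handle.
; Overlapping Exit removes the effect by that handle and re-arms the trigger.
; A shared WasTrigger flag prevents repeat application, so only one effect is tracked at a time.
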(event OnComponentBeginOverlap(Enter)
  (params (OverlappedComponent :type Primitive%20Component%20Object%20Reference) (OtherActor :type Actor%20Object%20Reference) (OtherComp :type Primitive%20Component%20Object%20Reference) (OtherBodyIndex :type Integer) (bFromSweep :type Boolean) (SweepResult :type Hit%20Result%20Structure%20%28by%20ref%29))
  (bind _asplayer_character (Utilities|Casting|CastToPlayerCharacter OtherActor))
  (if (not (Variables|Default|GetbWasTrigger))
    (Variables|Default|SetbWasTrigger true)
    (Utilities|IsValid (Ability|GetAbilitySystemComponent _asplayer_character)
      (:Is%20Valid
        (bind _returnvalue (GameplayEffects|ApplyGameplayEffectToSelf :self (Ability|GetAbilitySystemComponent _asplayer_character) :GameplayEffectClass "/Game/Core/GAS/Effects/Safe/GE_Safe.GE_Safe_C"))
        (Development|PrintString "safe")
        (Variables|Default|SetSafeHandle _returnvalue)))))

(event OnComponentBeginOverlap(Exit)
  (params (OverlappedComponent :type Primitive%20Component%20Object%20Reference) (OtherActor :type Actor%20Object%20Reference) (OtherComp :type Primitive%20Component%20Object%20Reference) (OtherBodyIndex :type Integer) (bFromSweep :type Boolean) (SweepResult :type Hit%20Result%20Structure%20%28by%20ref%29))
  (if (Variables|Default|GetbWasTrigger)
    (bind _asplayer_character (Utilities|Casting|CastToPlayerCharacter OtherActor))
    (Utilities|IsValid (Ability|GetAbilitySystemComponent _asplayer_character)
      (:Is%20Valid
        (GameplayEffects|RemoveActiveGameplayEffect (Ability|GetAbilitySystemComponent _asplayer_character) (Variables|Default|GetSafeHandle) -1)
        (Variables|Default|SetbWasTrigger false)))))

(fn ConstructionScript)